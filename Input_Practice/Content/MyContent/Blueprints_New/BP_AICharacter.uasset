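; Grid-based, multiplayer top-down character that moves, attacks tiles and reports its death to the game mode.
; The server turns it toward the attack target and multicasts linking of the attack's anim layers.
; Attack start, hit-frame and end events forward to OwningUser, while AttackPositions multicasts damage to other characters on attacked tiles.
; Grid and attack components supply movable and attackable tile highlights, and health component events refresh the health bar widget.
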(event `self.ReceiveTick`
  (params (DeltaSeconds :type "Float (single-precision)"))
  ;[0.05208 0.05208 0.05208 1 24] Event Tick
  (`self.MoveToDestination`))

(event `self.ReceiveBeginPlay`
  (bind _healthcomponent (`self.HealthComponent`))
  ;[0.05208 0.05208 0.05208 1 24] Event BeginPlay
  (set `self.TargetDestination` (`self.K2_GetActorLocation`))
  (add `AComp_Health.OnDeath` _healthcomponent (delegate `DeathEvent`))
  (`self.UpdateHealthWidget`)
  (add `AComp_Health.OnHit` _healthcomponent (delegate `HitEvent`))
  (add `AComp_Attack.OnAttackSet` (`self.AttackComponent`) (delegate `SetNewAttack`)))

(event `DeathEvent`
  ;[0.05208 0.05208 0.05208 1 24] Event Dispatch Bindings
  (bind _astop_down_game_mode (cast `/Game/MyContent/Core/TopDownGameMode` (`GameplayStatics.GetGameMode`)))
  (`/Game/MyContent/Core/TopDownGameMode.Destroy Character` _astop_down_game_mode self (`self.GetPlayerIndex`)))

(event `SetNewAttack`
  (params (NewAttack :type "DA_Attack Object Reference"))
  ;[0.05208 0.05208 0.05208 1 24] Event Dispatch Bindings
)

(event `HitEvent`
  ;[0.05208 0.05208 0.05208 1 24] Event Dispatch Bindings
  (`self.UpdateHealthWidget`))

(event `self.PrepareToStartAttack`
  (params (InAttack :type "DA_Attack Object Reference") (InputPos :type "Vector Structure"))
  (bind _capsulecomponent (`self.CapsuleComponent`))
  ;[0.05208 0.05208 0.05208 1 28] Link Anim Layers/Animation Notify Events
  ;;[1 0 0] Called From Server (C++)
  (if (`KismetSystemLibrary.IsServer`)
    (set `self.CurrentAttack` InAttack)
    (bind _output_get (set `self.AttackCursorPos` InputPos))
    (`SceneComponent.K2_SetWorldRotation` _capsulecomponent (`KismetMathLibrary.FindLookAtRotation` (`SceneComponent.K2_GetComponentLocation` _capsulecomponent) _output_get) false false :!label _label)
    (`self.ReplicateStartAnimation MULTI` (`DA_Attack.GetAnimInstance` (`self.CurrentAttack`)))
    (else
      (`KismetSystemLibrary.PrintString` "dfk?????????????????????" true true (struct :`R` 0.965246 :`G` 0.082091 :`B` 1.0 :`A` 1.0) 5.0)
      (`self.SERVER NOW` InAttack InputPos))))

(event `SERVER NOW`
  (params (InAttack :type "DA_Attack Object Reference") (InputPos :type "Vector Structure"))
  ;[0.05208 0.05208 0.05208 1 28] Link Anim Layers/Animation Notify Events
  ;;[1 0 0] Called From Server (C++)
  (set `self.CurrentAttack` InAttack)
  (set `self.AttackCursorPos` InputPos)
  (goto _label))

(event `self.PrepareToStopAttack`
  ;[0.05208 0.05208 0.05208 1 28] Link Anim Layers/Animation Notify Events
  ;;[1 0 0] Called From Server (C++)
  (`self.ReplicateStopAnimation MULTI` (`DA_Attack.GetAnimInstance` (`self.CurrentAttack`))))

(event `self.AttackPositions`
  (params (AttackedTiles :type "Array of Vector2D Structure (by ref)") (Damage :type Integer))
  ;[0.05208 0.05208 0.05208 1 36] Grid-related Input
  ;;[0.05208 0.05208 0.05208] Attacking Array of Positions (SERVER)
  (bind _ascpp_top_down_game_state (cast `CPP_TopDownGameState` (`GameplayStatics.GetGameState`)))
  (for _array_element AttackedTiles
    (bind (_foundcharacter _returnvalue) (`CPP_TopDownGameState.GetCharacterAtGridPosition` _ascpp_top_down_game_state _array_element))
    (if _returnvalue
      (if (!= _foundcharacter self)
        (`self.Event Take Damage MULTI` (`AICharacter.HealthComponent` _foundcharacter) Damage)))))

(event `ReplicateStartAnimation MULTI`
  (params (Attack :type "AnimInstance Class Reference"))
  ;[0.05208 0.05208 0.05208 1 28] Link Anim Layers/Animation Notify Events
  ;;[0 0.2 1] MultiCast From Server
  (if (`KismetSystemLibrary.IsValidClass` Attack)
    (`SkeletalMeshComponent.LinkAnimClassLayers` (`self.SkeletalMesh`) Attack)
    (else
      (`KismetSystemLibrary.PrintString` "CANNOT REPLICATE ANIMATION" true true (struct :`R` 0.45037 :`G` 0.221533 :`B` 1.0 :`A` 1.0) 5.0 :!label _label_2))))

(event `Event Take Damage MULTI`
  (params (HealthComp :type "AComp_Health Object Reference") (Damage :type Integer))
  ;[0.05208 0.05208 0.05208 1 36] Grid-related Input
  (`AComp_Health.TakeDamage` HealthComp Damage))

(event `self.ActivateMoveableTiles`
  (bind _gridcomponent (`self.GridComponent`))
  ;[0.05208 0.05208 0.05208 1 36] Grid-related Input
  ;;[0.05208 0.05208 0.05208] Display Navigable Tiles
  (bind _outtiles (`AComp_Grid.GetSurroundingTiles` _gridcomponent (`self.MoveRange`) false))
  (bind _asbp_grid (cast `/Game/MyContent/Blueprints_New/BP_Grid` (`AComp_Grid.GetGrid` _gridcomponent)))
  (`CPP_Grid.SetMoveableTilesPositions` _asbp_grid _outtiles))

(event `ReplicateStopAnimation MULTI`
  (params (Attack :type "AnimInstance Class Reference"))
  ;[0.05208 0.05208 0.05208 1 28] Link Anim Layers/Animation Notify Events
  ;;[0 0.2 1] MultiCast From Server
  (if (`KismetSystemLibrary.IsValidClass` Attack)
    (`SkeletalMeshComponent.UnlinkAnimClassLayers` (`self.SkeletalMesh`) Attack)
    (else
      (goto _label_2))))

(event `/Game/MyContent/Interfaces/INT_Attacker.AttackStarted`
  (params (AnimationDuration :type "Float (double-precision)"))
  (bind _owninguser (`self.OwningUser`))
  ;[0.05208 0.05208 0.05208 1 28] Link Anim Layers/Animation Notify Events
  (`/Engine/EditorBlueprintResources/StandardMacros.IsValid` _owninguser
    (:`Is Valid`
      (`KismetSystemLibrary.PrintString` "HAS VALID OWNING USER!" true true (struct :`G` 1.0 :`A` 1.0) 10.0)
      (`AComp_GridUser.AttackStarting` _owninguser))
    (:`Is Not Valid`
      (`KismetSystemLibrary.PrintString` "DOES NOT HAVE VALID OWNING USER!" true true (struct :`R` 1.0 :`G` 0.016606 :`A` 1.0) 10.0 :!label _label_3))))

(event `self.ActivateAttackableTiles`
  (bind _gridcomponent (`self.GridComponent`))
  (bind _returnvalue (`AComp_Grid.GetGrid` _gridcomponent))
  (bind (_outdamage _outisaoe _outattackrange _outattacktiles) (`AComp_Attack.GetAttackVariables` (`self.AttackComponent`)))
  ;[0.05208 0.05208 0.05208 1 36] Grid-related Input
  ;;[0.05729 0.05729 0.05729] Display Attackable Tiles
  (if _outisaoe
    (bind _outtiles (`AComp_Grid.GetAttackableTiles` _gridcomponent _outattacktiles (0.0 0.0 0.0)))
    (bind _asbp_grid (cast `/Game/MyContent/Blueprints_New/BP_Grid` _returnvalue))
    (`CPP_Grid.SetAttackableTilesPositions` _asbp_grid _outtiles)
    (else
      (bind _outtiles_2 (`AComp_Grid.GetSurroundingTiles` (`self.GridComponent`) _outattackrange true))
      (bind _asbp_grid_2 (cast `/Game/MyContent/Blueprints_New/BP_Grid` _returnvalue))
      (`CPP_Grid.SetAttackableTilesPositions` _asbp_grid_2 _outtiles_2))))

(event `/Game/MyContent/Interfaces/INT_Attacker.AttackEnded`
  (bind _owninguser (`self.OwningUser`))
  ;[0.05208 0.05208 0.05208 1 28] Link Anim Layers/Animation Notify Events
  (`/Engine/EditorBlueprintResources/StandardMacros.IsValid` _owninguser
    (:`Is Valid`
      (`KismetSystemLibrary.PrintString` "HAS VALID OWNING USER!" true true (struct :`G` 1.0 :`A` 1.0) 10.0)
      (`AComp_GridUser.AttackEnding` _owninguser self))
    (:`Is Not Valid`
      (goto _label_3))))

(event `/Game/MyContent/Interfaces/INT_Attacker.AttackThisFrame`
  ;[0.05208 0.05208 0.05208 1 28] Link Anim Layers/Animation Notify Events
  (`/Engine/EditorBlueprintResources/StandardMacros.IsValid` (`self.OwningUser`)
    (:`Is Valid`
      (`KismetSystemLibrary.PrintString` "HAS VALID OWNING USER!" true true (struct :`G` 1.0 :`A` 1.0) 10.0)
      (`AComp_GridUser.AttackThisFrame` (`self.OwningUser`) self (`self.CurrentAttack`) (`self.AttackCursorPos`)))
    (:`Is Not Valid`
      (goto _label_3))))

(fn `UpdateHealthWidget`
  (bind _healthcomponent (`self.HealthComponent`))
  (bind _aswb_health_bar (cast `/Game/MyContent/Blueprints_New/WB_HealthBar` (`WidgetComponent.GetUserWidgetObject` (`self.HealthWidget`))))
  (`/Engine/EditorBlueprintResources/StandardMacros.IsValid` _aswb_health_bar
    (:`Is Valid`
      (`/Game/MyContent/Blueprints_New/WB_HealthBar.SetHealthValues CLIENT` _aswb_health_bar (`AComp_Health.GetMaxHealth` _healthcomponent) (`AComp_Health.GetCurrentHealth` _healthcomponent)))
    (:`Is Not Valid`
      (`KismetSystemLibrary.PrintString` "invalid cast to WB_HealthBar"))))

(fn `UserConstructionScript`)