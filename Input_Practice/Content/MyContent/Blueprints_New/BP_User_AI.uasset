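; AI grid user for turn-based tactics that chooses and executes the selected character's move and attack.
; On turn start it maps opposing characters, then tests each reachable tile against targeted attacks and four-direction AOE attacks.
; It picks randomly among top distance-scored scenarios (computed damage and kill bonus never reach the score), else approaches the nearest enemy.
; HasMoved splits execution: move first, then attack or pass on the next call.
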(event `self.ReceiveBeginPlay`
  (bind _asbp_grid (cast `/Game/MyContent/Blueprints_New/BP_Grid` (`AComp_GridUser.Grid` (`self.UserComponent`))))
  (set `self.GridRef` _asbp_grid)
  (bind _asbp_core_top_down_game_state (cast `/Game/MyContent/Core/BP_Core_TopDownGameState` (`GameplayStatics.GetGameState`)))
  (set `self.GameStateRef` _asbp_core_top_down_game_state))

(event `StartNewTurn`
  (`KismetSystemLibrary.Delay` 1.0)
  (`|ExecutionSequence`
    (:`then_0`
      (bind _asbp_aicharacter (cast `/Game/MyContent/Blueprints_New/BP_AICharacter` (`AComp_GridUser.GetSelectedCharacter` (`self.UserComponent`)))
        (:`then`
          (bind _output_get (set `self.SelectedCharacter` _asbp_aicharacter))
          (bind _outtiles (`AComp_Grid.GetSurroundingTiles` (`AICharacter.GridComponent` _output_get) (`AICharacter.MoveRange` _output_get) false))
          (set `self.MoveableTiles` _outtiles))
        (:`CastFailed`
          (`KismetSystemLibrary.PrintString` "FAILED to get Selected Character from AI" true true (struct :`R` 1.0 :`A` 1.0) 10.0))))
    (:`then_1`
      (bind _returnvalue (`CPP_TopDownGameState.GetCharactersOwnedByPlayers` (`self.GameStateRef`) (select `int` (`AComp_GridUser.UserIndex` (`self.UserComponent`)) :`0` 1 :`1` 0)))
      (for _array_element _returnvalue
        (bind _asbp_aicharacter_2 (cast `/Game/MyContent/Blueprints_New/BP_AICharacter` _array_element))
        (`BlueprintMapLibrary.Map_Add` (`self.CharacterMap`) (`AComp_Grid.GetCurrentGridPosition` (`AICharacter.GridComponent` _array_element)) _asbp_aicharacter_2)))
    (:`then_2`
      (if (not (`self.HasMoved`))
        (bind _outscenario (`self.FindBestScenario`))
        (set `self.ChosenScenario` _outscenario)
        (`self.Execute Scenario`)
        (else
          (`self.Execute Scenario`))))))

(fn `CalculateAndSetScenarioScore`
  (params (InAttack :type "DA_Attack Object Reference") (InMovePos :type "Vector2D Structure") (`InAttackPos'` :type "Array of Vector2D Structure") (InAttackDir :type "E_CardinalDirection Enum" :default "CD_Up"))
  (returns (ScoredScenario :type "/Game/MyContent/Blueprints_New/S_Scenario Structure"))
  (locals (TempScore :type Integer) (ClosestAttackPosition :type "Vector2D Structure") (TempAttackPos :type "Vector2D Structure") (ClosestDistance :type "Float (double-precision)" :default 10000.0) (TempTotalDamage :type Integer))
  (bind _inattackpos_ (`local.InAttackPos'`))
  (bind _returnvalue (`DA_Attack.GetDamage` (`local.InAttack`)))
  (`|ExecutionSequence`
    (:`then_0`
      ;[0.04167 0.04167 0.04167 1 36] Get Closest Attack Position
      (if (<= (`KismetArrayLibrary.Array_Length` _inattackpos_) 1)
        (set `local.ClosestAttackPosition` (`|GetArrayItem` _inattackpos_))
        (else
          (for _array_element _inattackpos_
            (if (`.ReturnValue` (`BlueprintMapLibrary.Map_Find` (`self.CharacterMap`) _array_element))
              (bind _output_get (set `local.TempAttackPos` _array_element))
              (bind _returnvalue_2 (`KismetMathLibrary.Distance2D` _output_get (`local.InMovePos`)))
              (if (< _returnvalue_2 (`local.ClosestDistance`))
                (set `local.ClosestDistance` _returnvalue_2)
                (set `local.ClosestAttackPosition` (`local.TempAttackPos`))))))))
    (:`then_1`
      ;[0.05208 0.05208 0.05208 1 36] Set Score based on Attack tile distance
      (set `local.TempScore` (+ (`local.TempScore`) (* (`KismetMathLibrary.FTrunc` (* (`KismetMathLibrary.Distance2D` (`local.InMovePos`) (`local.ClosestAttackPosition`)) 100.0)) (`self.Factor_DistFromTarget`)))))
    (:`then_2`
      ;[0.04167 0.04167 0.04167 1 36] Set Score based on Damage dealt
      (for _array_element_2 (`local.InAttackPos'`)
        (bind (_value _returnvalue_3) (`BlueprintMapLibrary.Map_Find` (`self.CharacterMap`) _array_element_2))
        (if _returnvalue_3
          (set `local.TempTotalDamage` (+ (`local.TempTotalDamage`) (* (`self.Factor_DamageDealt`) (* _returnvalue 100))))
          ;;[0.04167 0.04167 0.04167] Fatal Attack
          (if (<= (- (`AComp_Health.GetCurrentHealth` (`AICharacter.HealthComponent` _value)) _returnvalue) 0)
            (set `local.TempTotalDamage` (+ (`local.TempTotalDamage`) 100000))))))
    (:`then_3`
      ;[0.05729 0.05729 0.05729 1 36] Return Scored Scenario
      (return (make `/Game/MyContent/Blueprints_New/S_Scenario` (`local.TempScore`) true (`local.InAttack`) (`local.InMovePos`) (`local.InAttackPos'`) (`local.InAttackDir`))))))

(fn `CalculateAndSetScenarioScore_Moving`
  (params (ClosestCharPos :type "Vector2D Structure") (MoveableTiles :type "Array of Vector2D Structure"))
  (returns (OutScenario :type "/Game/MyContent/Blueprints_New/S_Scenario Structure"))
  (locals (ClosestDist :type "Float (double-precision)") (ClosestPos :type "Vector2D Structure"))
  (for _array_element MoveableTiles
    (bind _returnvalue (`KismetMathLibrary.DistanceSquared2D` _array_element ClosestCharPos))
    (if (< _returnvalue (`local.ClosestDist`))
      (set `local.ClosestDist` _returnvalue)
      (set `local.ClosestPos` _array_element)))
  (return (make `/Game/MyContent/Blueprints_New/S_Scenario` 10 false null (`local.ClosestPos`) (`|MakeArray` (0.0 0.0) :!type "Vector2D Structure"))))

(fn `DoAttacksHitCharacters`
  (params (AllAttackPositions :type "Array of Vector2D Structure"))
  (returns (IsValid :type Boolean))
  (for _array_element AllAttackPositions
    (if (`.ReturnValue` (`BlueprintMapLibrary.Map_Find` (`self.CharacterMap`) _array_element))
      (return true)))
  (return false))

(fn `Execute Scenario`
  (bind _selectedcharacter (`self.SelectedCharacter`))
  (bind (_chosenscenario_scen_score _chosenscenario_action_isattacking _chosenscenario_action_attack _chosenscenario_action_tilemoveposition _chosenscenario_action_attackpositions _chosenscenario_action_attackdirection) (break `/Game/MyContent/Blueprints_New/S_Scenario` (`self.ChosenScenario`)))
  (bind _chosenscenario (`self.ChosenScenario`))
  (bind _returnvalue (`KismetMathLibrary.FTrunc` (`.Y` (`KismetMathLibrary.BreakVector2D` (`.Action_TileMovePosition_15_B1BA0B8C46231BFC50DA8B9C698F20BB` (break `/Game/MyContent/Blueprints_New/S_Scenario` _chosenscenario))))))
  (bind _returnvalue_2 (`CPP_Grid.GetTileSize` (`self.GridRef`)))
  (bind (_returnvalue_x _returnvalue_y _returnvalue_z) (`KismetMathLibrary.BreakVector` (`self.K2_GetActorLocation` _selectedcharacter)))
  (bind _returnvalue_3 (`self.K2_GetActorLocation` (`self.SelectedCharacter`)))
  (bind _returnvalue_4 (`KismetMathLibrary.FTrunc` (`KismetMathLibrary.BreakVector2D` (`.Action_TileMovePosition_15_B1BA0B8C46231BFC50DA8B9C698F20BB` (break `/Game/MyContent/Blueprints_New/S_Scenario` _chosenscenario)))))
  (bind (_output_x _output_y) (`KismetMathLibrary.BreakVector2D` (`|GetArrayItem` _chosenscenario_action_attackpositions)))
  (bind _returnvalue_5 (* _returnvalue_2 -1.0))
  (if (`self.HasMoved`)
    (set `self.HasMoved` false)
    (if _chosenscenario_action_isattacking
      (if (`DA_Attack.GetIsAOE` _chosenscenario_action_attack)
        (switch `E_CardinalDirection` _chosenscenario_action_attackdirection
          (:`CD_Up`
            (`AICharacter.Event_MultiRPC_PrepareAttack` (`self.SelectedCharacter`) _chosenscenario_action_attack (+ (`KismetMathLibrary.MakeVector` _returnvalue_2) _returnvalue_3)))
          (:`CD_Down`
            (`AICharacter.Event_MultiRPC_PrepareAttack` (`self.SelectedCharacter`) _chosenscenario_action_attack (+ (`KismetMathLibrary.MakeVector` _returnvalue_5) _returnvalue_3)))
          (:`CD_Right`
            (`AICharacter.Event_MultiRPC_PrepareAttack` (`self.SelectedCharacter`) _chosenscenario_action_attack (+ (`KismetMathLibrary.MakeVector` 0.0 _returnvalue_2) _returnvalue_3)))
          (:`CD_Left`
            (`AICharacter.Event_MultiRPC_PrepareAttack` (`self.SelectedCharacter`) _chosenscenario_action_attack (+ (`KismetMathLibrary.MakeVector` 0.0 _returnvalue_5) _returnvalue_3))))
        (else
          (bind _outgridlocation (`CPP_Grid.TileToGridWorldLocation` (`self.GridRef`) (`KismetMathLibrary.FTrunc` _output_x) (`KismetMathLibrary.FTrunc` _output_y) true))
          (`AICharacter.Event_MultiRPC_PrepareAttack` _selectedcharacter _chosenscenario_action_attack (`KismetMathLibrary.MakeVector` (`KismetMathLibrary.BreakVector2D` _outgridlocation) (`.Y` (`KismetMathLibrary.BreakVector2D` _outgridlocation)) _returnvalue_z))))
      (else
        (`AComp_GridUser.Event_ServerRPC_Pass` (`self.UserComponent`) "PA_Pass")))
    (else
      (bind (_outgridlocation_2 _returnvalue_6) (`CPP_Grid.TileToGridWorldLocation` (`self.GridRef`) _returnvalue_4 _returnvalue true))
      (if _returnvalue_6
        (set `self.HasMoved` true)
        (`AComp_GridUser.Event_ServerRPC_Move` (`self.UserComponent`) "PA_Move" (`KismetMathLibrary.MakeVector` (`KismetMathLibrary.BreakVector2D` _outgridlocation_2) (`.Y` (`KismetMathLibrary.BreakVector2D` _outgridlocation_2))))
        (`KismetSystemLibrary.PrintText` (`|FormatText` "Moving Toward Tile ({x},{y})!" _returnvalue_4 _returnvalue) true true (struct :`G` 1.0 :`B` 0.329394 :`A` 1.0) 15.0)))))

(fn `FindBestScenario`
  (returns (OutScenario :type "/Game/MyContent/Blueprints_New/S_Scenario Structure"))
  (locals (TempScenario :type "/Game/MyContent/Blueprints_New/S_Scenario Structure") (BestScenarios :type "Array of /Game/MyContent/Blueprints_New/S_Scenario Structure"))
  (bind _tempscenario_scen_score (break `/Game/MyContent/Blueprints_New/S_Scenario` (`local.TempScenario`)))
  (bind _bestscenarios (`local.BestScenarios`))
  (bind _tempscenario_scen_score_2 (break `/Game/MyContent/Blueprints_New/S_Scenario` (`local.TempScenario`)))
  (bind _bestscenarios_2 (`local.BestScenarios`))
  (bind _charactermap (`self.CharacterMap`))
  (bind _bestscenarios_3 (`local.BestScenarios`))
  (bind _returnvalue (`CPP_Grid.GetTileSize` (`self.GridRef`)))
  (bind _returnvalue_2 (`self.K2_GetActorLocation` (`self.SelectedCharacter`)))
  (bind _output_scen_score (break `/Game/MyContent/Blueprints_New/S_Scenario` (`|GetArrayItem` (`local.BestScenarios`))))
  (bind _output_scen_score_2 (break `/Game/MyContent/Blueprints_New/S_Scenario` (`|GetArrayItem` (`local.BestScenarios`))))
  (bind _returnvalue_3 (* _returnvalue -1.0))
  (`|ExecutionSequence`
    (:`then_0`
      (for _array_element (`self.MoveableTiles`)
        (if (`AICharacter.IsValidGridMovePosition` (`self.SelectedCharacter`) _array_element)
          (for _array_element_2 (`AComp_Attack.GetAttackList` (`AICharacter.AttackComponent` (`self.SelectedCharacter`)))
            (if (`DA_Attack.GetIsAOE` _array_element_2)
              ;[0.05729 0.05729 0.05729 1 36] Loop Over Character Positions for AOE Attacks
              (`|ExecutionSequence`
                (:`then_0`
                  (bind _returnvalue_4 (`DA_Attack.GetAttackTiles` _array_element_2))
                  (bind _outtiles (`AComp_Grid.GetAttackableTiles` (`AICharacter.GridComponent` (`self.SelectedCharacter`)) _returnvalue_4 (+ (`KismetMathLibrary.MakeVector` _returnvalue) _returnvalue_2)))
                  (if (`self.DoAttacksHitCharacters` _outtiles)
                    (bind _scoredscenario (`self.CalculateAndSetScenarioScore` _array_element_2 _array_element _outtiles))
                    ;;[0.05729 0.05729 0.05729 1 36] Adding Attack to Array
                    (set `local.TempScenario` _scoredscenario)
                    (if (> (`KismetArrayLibrary.Array_Length` (`local.BestScenarios`)) 0) :!label _label
                      (if (> _tempscenario_scen_score _output_scen_score)
                        (`KismetArrayLibrary.Array_Clear` _bestscenarios_3)
                        (`KismetArrayLibrary.Array_Add` _bestscenarios_3 (`local.TempScenario`) :!label _label_2)
                        (elif (== _tempscenario_scen_score _output_scen_score)
                          (goto _label_2)))
                      (else
                        (`KismetArrayLibrary.Array_Add` (`local.BestScenarios`) (`local.TempScenario`))))))
                (:`then_1`
                  (bind _outtiles_2 (`AComp_Grid.GetAttackableTiles` (`AICharacter.GridComponent` (`self.SelectedCharacter`)) _returnvalue_4 (+ (`KismetMathLibrary.MakeVector` _returnvalue_3) _returnvalue_2)))
                  (if (`self.DoAttacksHitCharacters` _outtiles_2)
                    (bind _scoredscenario_2 (`self.CalculateAndSetScenarioScore` _array_element_2 _array_element _outtiles_2 "CD_Down"))
                    (set `local.TempScenario` _scoredscenario_2)
                    (goto _label)))
                (:`then_2`
                  (bind _outtiles_3 (`AComp_Grid.GetAttackableTiles` (`AICharacter.GridComponent` (`self.SelectedCharacter`)) _returnvalue_4 (+ (`KismetMathLibrary.MakeVector` 0.0 _returnvalue) _returnvalue_2)))
                  (if (`self.DoAttacksHitCharacters` _outtiles_3)
                    (bind _scoredscenario_3 (`self.CalculateAndSetScenarioScore` _array_element_2 _array_element _outtiles_3 "CD_Right"))
                    (set `local.TempScenario` _scoredscenario_3)
                    (goto _label)))
                (:`then_3`
                  (bind _outtiles_4 (`AComp_Grid.GetAttackableTiles` (`AICharacter.GridComponent` (`self.SelectedCharacter`)) _returnvalue_4 (+ (`KismetMathLibrary.MakeVector` 0.0 _returnvalue_3) _returnvalue_2)))
                  (if (`self.DoAttacksHitCharacters` _outtiles_4)
                    (bind _scoredscenario_4 (`self.CalculateAndSetScenarioScore` _array_element_2 _array_element _outtiles_4 "CD_Left"))
                    (set `local.TempScenario` _scoredscenario_4)
                    (goto _label))))
              (else
                ;[0.04688 0.04688 0.04688 1 36] Loop over Character Positions for Targeted Attack
                (bind _keys (`BlueprintMapLibrary.Map_Keys` _charactermap))
                (for _array_element_3 _keys
                  (bind (_value _returnvalue_5) (`BlueprintMapLibrary.Map_Find` _charactermap _array_element_3))
                  (if _returnvalue_5
                    (if (`AICharacter.IsValidGridTarget` (`self.SelectedCharacter`) _value _array_element_3 _array_element (`DA_Attack.GetAttackRange` _array_element_2))
                      (bind _scoredscenario_5 (`self.CalculateAndSetScenarioScore` _array_element_2 _array_element (`|MakeArray` _array_element_3)))
                      (set `local.TempScenario` _scoredscenario_5)
                      (if (> (`KismetArrayLibrary.Array_Length` (`local.BestScenarios`)) 0)
                        (if (> _tempscenario_scen_score_2 _output_scen_score_2)
                          (`KismetArrayLibrary.Array_Clear` _bestscenarios_2)
                          (`KismetArrayLibrary.Array_Add` _bestscenarios_2 (`local.TempScenario`) :!label _label_3)
                          (elif (== _tempscenario_scen_score_2 _output_scen_score_2)
                            (goto _label_3)))
                        (else
                          (`KismetArrayLibrary.Array_Add` (`local.BestScenarios`) (`local.TempScenario`)))))))))))))
    (:`then_1`
      ;[0.05208 0.05208 0.05208 1 28] Change decision making if no worth-while Attacks were found
      (if (<= (`KismetArrayLibrary.Array_Length` (`local.BestScenarios`)) 0)
        (bind _outcharpos (`self.GetClosestCharacter`))
        (bind _outscenario (`self.CalculateAndSetScenarioScore_Moving` _outcharpos (`self.MoveableTiles`)))
        (`KismetArrayLibrary.Array_Add` (`local.BestScenarios`) _outscenario)))
    (:`then_2`
      ;[0.05208 0.05208 0.05208] Get Random Scenario from the BEST Scenarios
      (return (`|GetArrayItem` _bestscenarios (`KismetMathLibrary.RandomIntegerInRange` 0 (- (`KismetArrayLibrary.Array_Length` _bestscenarios) 1)))))))

(fn `GetClosestCharacter`
  (returns (OutCharPos :type "Vector2D Structure") (OutChar :type "/Game/MyContent/Blueprints_New/BP_AICharacter Object Reference"))
  (locals (ClosestDist :type "Float (double-precision)" :default -100000.0) (ClosestPos :type "Vector2D Structure") (SelectedPos :type "Vector2D Structure"))
  (bind _closestpos (`local.ClosestPos`))
  (set `local.SelectedPos` (`AComp_Grid.GetCurrentGridPosition` (`AICharacter.GridComponent` (`self.SelectedCharacter`))))
  (bind _keys (`BlueprintMapLibrary.Map_Keys` (`self.CharacterMap`)))
  (for _array_element _keys
    (bind _returnvalue (`KismetMathLibrary.Distance2D` _array_element (`local.SelectedPos`)))
    (if (< _returnvalue (`local.ClosestDist`))
      (set `local.ClosestDist` _returnvalue)
      (set `local.ClosestPos` _array_element)))
  (return _closestpos (`BlueprintMapLibrary.Map_Find` (`self.CharacterMap`) _closestpos)))

(fn `GetGridUser`
  (returns (ReturnValue :type "AComp_GridUser Object Reference"))
  (return (`self.UserComponent`)))

(fn `OnTurnEnd`)

(fn `OnTurnStart`
  (`self.StartNewTurn`))

(fn `UserConstructionScript`)