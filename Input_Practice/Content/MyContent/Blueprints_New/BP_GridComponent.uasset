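; BP_GridComponent records which tile of the game mode's grid its owning actor starts on.
; On BeginPlay it gets the grid from BP_TopDownGameMode, finds the tile under the owner and, if valid, takes that tile's non-centered location.
; ConvertVectorToGrid2D turns that location into grid coordinates using grid origin, tile size and a fixed offset.
; SetGridPosition stores the result and prints the floored coordinates for debugging, without moving the actor.
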(event `self.ReceiveBeginPlay`
  (set `self.Owner` (`self.GetOwner`))
  (bind _asbp_top_down_game_mode (cast `/Game/MyContent/Blueprints_New/BP_TopDownGameMode` (`GameplayStatics.GetGameMode`)))
  (bind _grid (`/Game/MyContent/Blueprints_New/BP_TopDownGameMode.GetGrid` _asbp_top_down_game_mode))
  (bind _output_get (set `self.Grid` _grid))
  (bind (_isvalid _row _column) (`/Game/MyContent/Blueprints_New/BP_Grid.LocationToTile` _output_get (`Actor.K2_GetActorLocation` (`self.Owner`))))
  (if _isvalid
    (bind (_isvalid_2 _gridlocation) (`/Game/MyContent/Blueprints_New/BP_Grid.TileToGridLocation` _grid _row _column false))
    (`self.SetGridPosition` (`self.ConvertVectorToGrid2D` _grid (`KismetMathLibrary.BreakVector2D` _gridlocation) (`.Y` (`KismetMathLibrary.BreakVector2D` _gridlocation))))))

(fn `ConvertVectorToGrid2D`
  (params (GridInfo :type "/Game/MyContent/Blueprints_New/BP_Grid Object Reference") (xPos :type "Float (double-precision)") (yPos :type "Float (double-precision)"))
  (returns (Vector2DPos :type "Vector2D Structure"))
  (bind (_returnvalue_x _returnvalue_y) (`KismetMathLibrary.BreakVector` (`Actor.K2_GetActorLocation` GridInfo)))
  (bind _returnvalue (/ (`/Game/MyContent/Blueprints_New/BP_Grid.TileSize` GridInfo) 100.0))
  (return (`KismetMathLibrary.MakeVector2D` (/ (- (/ (- xPos _returnvalue_x) 100.0) 1.0) _returnvalue) (/ (- (/ (- yPos _returnvalue_y) 100.0) 1.0) _returnvalue))))

(fn `SetGridPosition`
  (params (NewPosition :type "Vector2D Structure"))
  (bind _output_get (set `self.GridPosition` NewPosition))
  (`KismetSystemLibrary.PrintString` (`KismetTextLibrary.Conv_TextToString` (`|FormatText` "Current Tile: ({x},{y})" (`KismetMathLibrary.FFloor` (`KismetMathLibrary.BreakVector2D` _output_get)) (`KismetMathLibrary.FFloor` (`.Y` (`KismetMathLibrary.BreakVector2D` _output_get)))))))