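; Player pawn for a turn-based grid tactics game, turning cursor input into move and attack actions through UserComponent.
; Tick highlights the hovered tile or AOE area on the grid; clicks on the player's turn validate tiles, then send moves by server RPC and attacks by multicast, relayed through CallingtoSERVER on clients.
; It also manages lobby, gameplay and game-over widgets, starting an AI match when the level is not networked.
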(event `StartGameplay`
  (bind _startingui (`self.StartingUI`))
  ;[0.05208 0.05208 0.05208 1 36] Initialise Variables on Game Start
  (`/Engine/EditorBlueprintResources/StandardMacros.IsValid` _startingui
    (:`Is Valid`
      (clear `/Game/MyContent/Blueprints/WB_Start.OnLeaveBtnPressed` _startingui)
      (`Widget.RemoveFromParent` _startingui))
    (:`Is Not Valid`
      _))
  (if (`Controller.IsLocalController` (`self.GetController`))
    (bind _returnvalue (`|CreateWidget` "/Game/MyContent/Blueprints/WB_Gameplay.WB_Gameplay_C" (`GameplayStatics.GetPlayerController` 0)))
    (bind _output_get (set `self.PlayerUI` _returnvalue))
    (`UserWidget.AddToViewport` _output_get 0)
    (add `/Game/MyContent/Blueprints/WB_Gameplay.OnTurnModeToggled` _output_get (delegate `StateToggled`))
    (add `/Game/MyContent/Blueprints/WB_Gameplay.OnTurnEnd` _output_get (delegate `TurnEnding`))
    (`GameplayStatics.PlaySound2D` "/Game/MyContent/Sounds/Music.Music" 1.0 1.0 0.0 null null)))

(event `TurnEnding`
  ;[0.05208 0.05208 0.05208 1 36] Initialise Variables on Game Start
  (`AComp_GridUser.Event_ServerRPC_Pass` (`self.UserComponent`) "PA_Pass"))

(event `StateToggled`
  (params (NewState :type "E_PlayerActions Enum" :default "PA_Pass"))
  ;[0.05208 0.05208 0.05208 1 36] Initialise Variables on Game Start
  (`AComp_GridUser.StateToggle` (`self.UserComponent`) NewState))

(event `self.ReceiveBeginPlay`
  ;[0.05729 0.05729 0.05729 1 36] On Begin/End Play
  (if (`Controller.IsLocalController` (`self.GetController`))
    (`EnhancedInputSubsystemInterface.AddMappingContext` (pcsubsystem `EnhancedInputLocalPlayerSubsystem` (`GameplayStatics.GetPlayerController` 0)) "/Game/MyContent/Input_New/IMC_TopDown.IMC_TopDown" 0 (struct))
    (bind _ascpp_top_down_game_mode (cast `CPP_TopDownGameMode` (`GameplayStatics.GetGameMode`)))
    (bind _output_get (set `self.IsNetworking` (`CPP_TopDownGameMode.bIsNetworkedLevel` _ascpp_top_down_game_mode)))
    (if _output_get
      (bind _returnvalue (`|CreateWidget` "/Game/MyContent/Blueprints/WB_Start.WB_Start_C" (`GameplayStatics.GetPlayerController` 0)))
      (bind _output_get_2 (set `self.StartingUI` _returnvalue))
      (`UserWidget.AddToViewport` _output_get_2 0)
      (add `/Game/MyContent/Blueprints/WB_Start.OnLeaveBtnPressed` _output_get_2 (delegate `Leave Game`))
      (else
        (`CPP_TopDownGameMode.StartGameWithAI` _ascpp_top_down_game_mode)))))

(event `self.ReceiveTick`
  (params (DeltaSeconds :type "Float (single-precision)"))
  ;[0.04167 0.04167 0.04167 1 36] Player Input
  ;;[0.05208 0.05208 0.05208] Selected Tile On TICK
  (`self.UpdateCursorPosition`))

(event `EnhancedInput|/Game/MyContent/Input_New/Actions/IA_TopDown_Mouse_Click`
  (params (ActionValue :type Boolean) (ElapsedSeconds :type "Float (double-precision)") (TriggeredSeconds :type "Float (double-precision)") (InputAction :type "InputAction Object Reference" :default "/Game/MyContent/Input_New/Actions/IA_TopDown_Mouse_Click.IA_TopDown_Mouse_Click"))
  (bind _usercomponent (`self.UserComponent`))
  ;[0.04167 0.04167 0.04167 1 36] Player Input
  ;;[0.05208 0.05208 0.05208] Mouse Click on GRID
  (:`Completed`
    (if (and (`AComp_GridUser.IsMyTurn` _usercomponent) (not (`AComp_GridUser.HasPerformedFinalInput` _usercomponent)))
      (`self.HandleInputAction`))))

(event `self.ReceiveEndPlay`
  (params (EndPlayReason :type "EEndPlayReason Enum" :default "Destroyed"))
  (bind _playerui (`self.PlayerUI`))
  ;[0.05729 0.05729 0.05729 1 36] On Begin/End Play
  (`/Engine/EditorBlueprintResources/StandardMacros.IsValid` _playerui
    (:`Is Valid`
      (clear `/Game/MyContent/Blueprints/WB_Gameplay.OnTurnModeToggled` _playerui))))

(event `Leave Game`
  ;[0.05729 0.05729 0.05729 1 36] On Begin/End Play
  (bind _asbp_core_gs (cast `/Game/MyContent/Core/BP_Core_GS` (`GameplayStatics.GetGameState`)))
  (if (not (`/Game/MyContent/Core/BP_Core_GS.IsGameStarting` _asbp_core_gs))
    (`DestroySessionCallbackProxy.DestroySession` (`GameplayStatics.GetPlayerController` 0)
      (:`OnSuccess`
        (`GameplayStatics.OpenLevel` "L_MainMenu")))))

(event `GameOver`
  (params (IsWinner :type Boolean))
  ;[0.04688 0.04688 0.04688 1 36] Game Over
  (bind _returnvalue (`|CreateWidget` "/Game/MyContent/Blueprints/WB__GameOver.WB__GameOver_C" (`GameplayStatics.GetPlayerController` 0)))
  (`/Game/MyContent/Blueprints/WB__GameOver.SetGameOverValues` _returnvalue IsWinner)
  (`UserWidget.AddToViewport` _returnvalue 0)
  (`WidgetBlueprintLibrary.SetInputMode_UIOnlyEx` (`GameplayStatics.GetPlayerController` 0) _returnvalue)
  (`GameplayStatics.SetGamePaused` true))

(event `Calling to SERVER`
  (params (Character :type "AICharacter Object Reference") (Attack :type "DA_Attack Object Reference") (InputPos :type "Vector Structure"))
  ;[0.04167 0.04167 0.04167 1 36] Player Input
  ;;[0.05729 0.05729 0.05729] Server call for Remote Client
  (`AICharacter.Event_MultiRPC_PrepareAttack` Character Attack InputPos))

(fn `GetGridUser`
  (returns (ReturnValue :type "AComp_GridUser Object Reference"))
  (return (`self.UserComponent`)))

(fn `GetPositionFromCursorCast`
  (returns (ValidCast :type Boolean) (Position :type "Vector Structure"))
  (bind (_hitresult _returnvalue) (`PlayerController.GetHitResultUnderCursorByChannel` (`GameplayStatics.GetPlayerController` 0) "TraceTypeQuery1" true))
  (return _returnvalue (`.Location` (`GameplayStatics.BreakHitResult` _hitresult))))

(fn `HandleInputAction`
  (returns (WasActionTaken :type Boolean))
  (bind _grid (`AComp_GridUser.Grid` (`self.UserComponent`)))
  (bind _selectedcharacter (`AComp_GridUser.SelectedCharacter` (`self.UserComponent`)))
  (bind _returnvalue (`AComp_Attack.GetAttack` (`AICharacter.AttackComponent` _selectedcharacter)))
  (bind (_outdamage _outisaoe _outattackrange) (`AComp_Attack.GetAttackVariables` (`AICharacter.AttackComponent` (`AComp_GridUser.SelectedCharacter` (`self.UserComponent`)))))
  (switch `E_PlayerActions` (`AComp_GridUser.CurrentState` (`self.UserComponent`))
    (:`PA_Move`
      ;[0.04688 0.04688 0.04688 1 28] Move Character to Position
      (bind (_validcast _position) (`self.GetPositionFromCursorCast`))
      (bind (_outworldposition _outgridposition _returnvalue_2) (`CPP_Grid.VectorToTile` (`AComp_GridUser.Grid` (`self.UserComponent`)) _position))
      (if _returnvalue_2
        (if (`AICharacter.IsValidGridMovePosition` (`AComp_GridUser.SelectedCharacter` (`self.UserComponent`)) _outgridposition)
          (`GameplayStatics.PlaySound2D` "/Game/MyContent/Sounds/select.select" 1.0 1.0 0.0 null null)
          (`AComp_GridUser.Event_ServerRPC_Move` (`self.UserComponent`) "PA_Move" _outworldposition)
          (return true)
          (else
            _)))
      (return false))
    (:`PA_Attack`
      ;[0.05208 0.05208 0.05208 1 28] Checks if Attacks are Valid
      (bind (_validcast_2 _position_2) (`self.GetPositionFromCursorCast`))
      (if _outisaoe
        (bind (_outworldposition_2 _outgridposition_2 _returnvalue_3) (`CPP_Grid.VectorToTile` _grid _position_2))
        (if _returnvalue_3
          _
          (else
            (return false)))
        (else
          (bind (_outworldposition_3 _outgridposition_3 _returnvalue_4) (`CPP_Grid.VectorToTile` _grid _position_2))
          (if _returnvalue_4
            (if (`AICharacter.IsValidGridTargetPosition` (`AComp_GridUser.SelectedCharacter` (`self.UserComponent`)) _outgridposition_3 _outattackrange)
              _
              (else
                (return false)))
            (else
              (return false)))))
      ;[0.04688 0.04688 0.04688 1 28] Executes Animations and Attacks on Server
      (`AComp_GridUser.SetHasPerformedFinalInput` (`self.UserComponent`) true)
      (bind (_validcast_3 _position_3) (`self.GetPositionFromCursorCast`))
      (`/Engine/EditorBlueprintResources/ActorMacros.Switch Has Authority`
        (:`Authority`
          (`AICharacter.Event_MultiRPC_PrepareAttack` _selectedcharacter _returnvalue _position_3)
          (return true))
        (:`Remote`
          (`self.Calling to SERVER` _selectedcharacter _returnvalue _position_3))))))

(fn `UpdateCursorPosition`
  (locals (SelectedAttack :type " Structure"))
  (bind _usercomponent (`self.UserComponent`))
  (bind _usercomponent_2 (`self.UserComponent`))
  (bind _selectedcharacter (`AComp_GridUser.SelectedCharacter` _usercomponent_2))
  (bind _grid (`AComp_GridUser.Grid` (`self.UserComponent`)))
  (if (`|EnumEquality` (`AComp_GridUser.CurrentState` _usercomponent) "PA_Attack")
    (if (`.OutIsAOE` (`AComp_Attack.GetAttackVariables` (`AICharacter.AttackComponent` (`AComp_GridUser.SelectedCharacter` _usercomponent))))
      ;[0.05729 0.05729 0.05729 1 36] Attacking AOE On Tick
      (`/Engine/EditorBlueprintResources/StandardMacros.IsValid` (`AComp_GridUser.Grid` _usercomponent_2)
        (:`Is Valid`
          (bind (_validcast _position) (`self.GetPositionFromCursorCast`))
          (bind _outtiles (`AComp_Grid.GetAttackableTiles` (`AICharacter.GridComponent` _selectedcharacter) (`.OutAttackTiles` (`AComp_Attack.GetAttackVariables` (`AICharacter.AttackComponent` _selectedcharacter))) _position))
          (`CPP_Grid.SetAttackableTilesPositions` (`AComp_GridUser.Grid` (`self.UserComponent`)) _outtiles)))
      (else
        ;[0.04688 0.04688 0.04688 1 36] Moving/Attacking-Target Mode On Tick
        (`/Engine/EditorBlueprintResources/StandardMacros.IsValid` _grid :!label _label
          (:`Is Valid`
            (bind (_validcast_2 _position_2) (`self.GetPositionFromCursorCast`))
            (if _validcast_2
              (bind (_outrow _outcolumn) (`CPP_Grid.LocationToTile` _grid _position_2))
              (`CPP_Grid.SetSelectedTilePosition` _grid _outrow _outcolumn)
              (else
                (`CPP_Grid.SetSelectedTilePosition` _grid -1 -1)))))))
    (else
      (goto _label))))

(fn `UserConstructionScript`)