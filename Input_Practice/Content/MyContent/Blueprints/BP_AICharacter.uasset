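; AI-controlled character for a grid-based, multiplayer top-down tactics game that moves to a destination and attacks tiles.
; Health component events refresh the health bar and have the game mode destroy it on death.
; Anim notify events forward attack timing to the owning user on authority, and tile attacks multicast damage.
; Grid and attack components supply highlighted move/attack tiles, while a RepNotify links and unlinks attack anim layers.
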(event `self.ReceiveTick`
  (params (DeltaSeconds :type "Float (single-precision)"))
  ;[0.05208 0.05208 0.05208 1 24] Event Tick
  (`self.MoveToDestination`))

(event `self.ReceiveBeginPlay`
  (bind _healthcomponent (`self.HealthComponent`))
  ;[0.05208 0.05208 0.05208 1 24] Event BeginPlay
  (set `self.TargetDestination` (`self.K2_GetActorLocation`))
  (add `AComp_Health.OnDeath` _healthcomponent (delegate `DeathEvent`))
  (`self.UpdateHealthWidget`)
  (add `AComp_Health.OnHit` _healthcomponent (delegate `HitEvent`))
  (add `AComp_Attack.OnAttackSet` (`self.AttackComponent`) (delegate `SetNewAttack`))
  (set `self.CharSkeletalMesh` (`self.SkeletalMesh`)))

(event `DeathEvent`
  ;[0.05208 0.05208 0.05208 1 24] Event Dispatch Bindings
  (bind _ascpp_top_down_game_mode (cast `CPP_TopDownGameMode` (`GameplayStatics.GetGameMode`)))
  (`CPP_TopDownGameMode.DestroyCharacter` _ascpp_top_down_game_mode self (`self.GetPlayerIndex`)))

(event `SetNewAttack`
  (params (NewAttack :type "DA_Attack Object Reference"))
  ;[0.05208 0.05208 0.05208 1 24] Event Dispatch Bindings
)

(event `HitEvent`
  ;[0.05208 0.05208 0.05208 1 24] Event Dispatch Bindings
  (`self.UpdateHealthWidget`))

(event `self.BindAttackAnim`
  (params (InAnim :type "AnimInstance Class Reference"))
  ;[0.05208 0.05208 0.05208 1 28] Link Anim Layers/Animation Notify Events
  ;;[0 0.2 1] MultiCast From Server
  (if (`KismetSystemLibrary.IsValidClass` InAnim)
    (set `self.CurrentAnim` InAnim)))

(event `self.UnbindAttackAnim`
  (params (InAnim :type "AnimInstance Class Reference"))
  ;[0.05208 0.05208 0.05208 1 28] Link Anim Layers/Animation Notify Events
  ;;[0 0.2 1] MultiCast From Server
  (if (`KismetSystemLibrary.IsValidClass` InAnim)
    (set `self.CurrentAnim` null)))

(event `self.AttackPositions`
  (params (AttackedTiles :type "Array of Vector2D Structure (by ref)") (Damage :type Integer))
  ;[0.05208 0.05208 0.05208 1 36] Grid-related Input
  ;;[0.05208 0.05208 0.05208] Attacking Array of Positions (SERVER)
  (bind _ascpp_top_down_game_state (cast `CPP_TopDownGameState` (`GameplayStatics.GetGameState`)))
  (for _array_element AttackedTiles
    (bind (_foundcharacter _returnvalue) (`CPP_TopDownGameState.GetCharacterAtGridPosition` _ascpp_top_down_game_state _array_element))
    (if _returnvalue
      (if (!= _foundcharacter self)
        (`self.Event Take Damage MULTI` (`AICharacter.HealthComponent` _foundcharacter) Damage)))))

(event `/Game/MyContent/Interfaces/INT_Attacker.AttackStarted`
  (params (AnimationDuration :type "Float (double-precision)"))
  ;[0.05208 0.05208 0.05208 1 28] Link Anim Layers/Animation Notify Events
  ;;[0.005214 1 0] Animation Events
  (`self.IsUserValid`
    (:`Is Valid`
      (`/Engine/EditorBlueprintResources/ActorMacros.Switch Has Authority`
        (:`Authority`
          (`AComp_GridUser.AttackStarting` (`self.OwningUser`)))))))

(event `/Game/MyContent/Interfaces/INT_Attacker.AttackThisFrame`
  ;[0.05208 0.05208 0.05208 1 28] Link Anim Layers/Animation Notify Events
  ;;[0.005214 1 0] Animation Events
  (`self.IsUserValid`
    (:`Is Valid`
      (`/Engine/EditorBlueprintResources/ActorMacros.Switch Has Authority`
        (:`Authority`
          (`AComp_GridUser.AttackThisFrame` (`self.OwningUser`) self (`self.Server_Attack`) (`self.Server_InputPos`)))))))

(event `Event Take Damage MULTI`
  (params (HealthComp :type "AComp_Health Object Reference") (Damage :type Integer))
  ;[0.05208 0.05208 0.05208 1 36] Grid-related Input
  (`AComp_Health.TakeDamage` HealthComp Damage)
  (`GameplayStatics.PlaySound2D` "/Game/MyContent/Sounds/hit.hit" 1.0 1.0 0.0 null null))

(event `self.ActivateMoveableTiles`
  (bind _gridcomponent (`self.GridComponent`))
  ;[0.05208 0.05208 0.05208 1 36] Grid-related Input
  ;;[0.05208 0.05208 0.05208] Display Navigable Tiles
  (bind _outtiles (`AComp_Grid.GetSurroundingTiles` _gridcomponent (`self.MoveRange`) false))
  (bind _asbp_grid (cast `/Game/MyContent/Blueprints/BP_Grid` (`AComp_Grid.GetGrid` _gridcomponent)))
  (`CPP_Grid.SetMoveableTilesPositions` _asbp_grid _outtiles))

(event `/Game/MyContent/Interfaces/INT_Attacker.AttackEnded`
  ;[0.05208 0.05208 0.05208 1 28] Link Anim Layers/Animation Notify Events
  ;;[0.005214 1 0] Animation Events
  (`self.IsUserValid`
    (:`Is Valid`
      (`/Engine/EditorBlueprintResources/ActorMacros.Switch Has Authority`
        (:`Authority`
          (`AComp_GridUser.AttackEnding` (`self.OwningUser`) self))))))

(event `self.ActivateAttackableTiles`
  (bind _gridcomponent (`self.GridComponent`))
  (bind _returnvalue (`AComp_Grid.GetGrid` _gridcomponent))
  (bind (_outdamage _outisaoe _outattackrange _outattacktiles) (`AComp_Attack.GetAttackVariables` (`self.AttackComponent`)))
  ;[0.05208 0.05208 0.05208 1 36] Grid-related Input
  ;;[0.05729 0.05729 0.05729] Display Attackable Tiles
  (if _outisaoe
    (bind _outtiles (`AComp_Grid.GetAttackableTiles` _gridcomponent _outattacktiles (0.0 0.0 0.0)))
    (bind _asbp_grid (cast `/Game/MyContent/Blueprints/BP_Grid` _returnvalue))
    (`CPP_Grid.SetAttackableTilesPositions` _asbp_grid _outtiles)
    (else
      (bind _outtiles_2 (`AComp_Grid.GetSurroundingTiles` (`self.GridComponent`) _outattackrange true))
      (bind _asbp_grid_2 (cast `/Game/MyContent/Blueprints/BP_Grid` _returnvalue))
      (`CPP_Grid.SetAttackableTilesPositions` _asbp_grid_2 _outtiles_2))))

(fn `OnRep_CurrentAnim`
  (bind _skeletalmesh (`self.SkeletalMesh`))
  (bind _currentanim (`self.CurrentAnim`))
  (if (`KismetSystemLibrary.IsValidClass` (`self.CurrentAnim`))
    (if (!= (`self.CurrentAnim`) (`self.PreviousAnim`))
      (if (`KismetSystemLibrary.IsValidClass` (`self.PreviousAnim`))
        (`SkeletalMeshComponent.UnlinkAnimClassLayers` _skeletalmesh (`self.PreviousAnim`)))
      (`SkeletalMeshComponent.LinkAnimClassLayers` _skeletalmesh _currentanim)
      (set `self.PreviousAnim` _currentanim))
    (elif (`KismetSystemLibrary.IsValidClass` (`self.PreviousAnim`))
      (`SkeletalMeshComponent.UnlinkAnimClassLayers` _skeletalmesh (`self.PreviousAnim`))
      (set `self.PreviousAnim` null))))

(fn `UpdateHealthWidget`
  (bind _healthcomponent (`self.HealthComponent`))
  (bind _aswb_health_bar (cast `/Game/MyContent/Blueprints/WB_HealthBar` (`WidgetComponent.GetUserWidgetObject` (`self.HealthWidget`))))
  (`/Engine/EditorBlueprintResources/StandardMacros.IsValid` _aswb_health_bar
    (:`Is Valid`
      (`/Game/MyContent/Blueprints/WB_HealthBar.SetHealthValues CLIENT` _aswb_health_bar (`AComp_Health.GetMaxHealth` _healthcomponent) (`AComp_Health.GetCurrentHealth` _healthcomponent)))
    (:`Is Not Valid`
      (`KismetSystemLibrary.PrintString` "invalid cast to WB_HealthBar"))))

(fn `UserConstructionScript`)