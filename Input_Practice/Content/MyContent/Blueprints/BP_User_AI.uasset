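; AI-controlled grid user that plays its own turns by choosing and executing a scored scenario.
; OnTurnStart triggers StartNewTurn, which waits briefly, initializes dynamic variables, then, if not yet moved, picks the best scenario, prints its score, executes it and plays a select sound.
; If already moved, it executes the stored scenario, then resets it to a very low-score placeholder.
; Scenario search and execution logic are defined outside this file.
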(event `self.StartNewTurn`
  (`KismetSystemLibrary.Delay` 1.0)
  (`self.InitialiseDynamicVariables`)
  (if (not (`self.bHasMoved`))
    (bind _returnvalue (`self.FindBestScenario`))
    (set `self.ChosenScenario` _returnvalue)
    (`KismetSystemLibrary.PrintString` (`KismetStringLibrary.Concat_StrStr` "CHOSEN Scenario Score: " (`KismetStringLibrary.Conv_IntToString` (`.Score` (break `Scenario` (`self.ChosenScenario`))))) true true (struct :`R` 0.515946 :`G` 0.251593 :`B` 1.0 :`A` 1.0) 15.0)
    (`self.ExecuteScenario`)
    (`GameplayStatics.PlaySound2D` "/Game/MyContent/Sounds/select.select" 1.0 1.0 0.0 null null)
    (else
      (`self.ExecuteScenario`)
      (set `self.ChosenScenario` (make `Scenario` -10000)))))

(fn `GetGridUser`
  (returns (ReturnValue :type "AComp_GridUser Object Reference"))
  (return (`self.UserComponent`)))

(fn `OnTurnEnd`)

(fn `OnTurnStart`
  (`self.StartNewTurn`))

(fn `UserConstructionScript`)