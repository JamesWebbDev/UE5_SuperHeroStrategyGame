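; Actor component that places its owner on the level's BP_Grid and tracks its tile position.
; On BeginPlay it finds the grid, converts the owner's location to a tile and snaps the owner to that tile's center at grid height.
; GetMoveableTiles gathers offsets within a Euclidean move radius, excluding the origin, without checking grid bounds or occupancy.
; GetAttackableTiles is an empty stub, and the origin/diagonal helper is unused here.
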(event `self.ReceiveBeginPlay`
  (set `self.Owner` (`self.GetOwner`))
  (bind _returnvalue (`GameplayStatics.GetActorOfClass` "/Game/MyContent/Blueprints_New/BP_Grid.BP_Grid_C"))
  (set `self.Grid` _returnvalue)
  (`self.SetGridPosition` (`self.GetCurrentLocationToTile`))
  (`self.SetWorldPositionFromGridPosition`))

(fn `GetAttackableTiles`
  (params (AffectedTiles_UpDirection :type "Array of Vector2D Structure"))
  (returns (TileLocations :type "Array of Vector2D Structure"))
  (return))

(fn `GetCurrentGridPosition`
  (returns (GridPosition :type "Vector2D Structure"))
  (return (`self.GridPosition`)))

(fn `GetCurrentLocationToTile`
  (returns (GridLocation :type "Vector2D Structure"))
  (bind _grid (`self.Grid`))
  (`/Engine/EditorBlueprintResources/StandardMacros.IsValid` _grid
    (:`Is Valid`
      (bind (_isvalid _row _column) (`/Game/MyContent/Blueprints_New/BP_Grid.LocationToTile` _grid (`Actor.K2_GetActorLocation` (`self.Owner`))))
      (if _isvalid
        (return (`KismetMathLibrary.MakeVector2D` (`KismetMathLibrary.Conv_IntToDouble` _row) (`KismetMathLibrary.Conv_IntToDouble` _column)))
        (else
          (`KismetSystemLibrary.PrintString` "ACTOR is not in valid location for grid ref"))))))

(fn `GetGrid`
  (returns (Grid :type "/Game/MyContent/Blueprints_New/BP_Grid Object Reference"))
  (return (`self.Grid`)))

(fn `GetMoveableTiles`
  (params (Move :type Integer))
  (returns (`Tile Locations` :type "Array of Vector2D Structure"))
  (locals (TileArray :type "Array of Vector2D Structure") (NegativeMove :type Integer) (XValue :type Integer) (YValue :type Integer) (TempGridPosition :type "Vector2D Structure") (Origin :type "Vector2D Structure"))
  (bind (_origin_x _origin_y) (`KismetMathLibrary.BreakVector2D` (`local.Origin`)))
  (set `local.Origin` (`self.GetCurrentLocationToTile`))
  (bind _output_get (set `local.NegativeMove` (* -1 (`local.Move`))))
  (for _index (range _output_get (+ (`local.Move`) 1))
    (set `local.XValue` _index)
    (for _index_2 (range (`local.NegativeMove`) (+ (`local.Move`) 1))
      (set `local.YValue` _index_2)
      (bind _output_get_2 (set `local.TempGridPosition` (`KismetMathLibrary.MakeVector2D` (+ _origin_x (`local.XValue`)) (+ _origin_y (`local.YValue`)))))
      (bind _returnvalue (`KismetMathLibrary.Distance2D` _output_get_2 (`local.Origin`)))
      (if (and (> _returnvalue 0.0) (<= _returnvalue (`local.Move`)))
        (`KismetArrayLibrary.Array_Add` (`local.TileArray`) (`local.TempGridPosition`)))))
  ;[0.05208 0.05208 0.05208 1 12] Runs when all Tiles have been checked
  (return (`local.TileArray`)))

(fn `IsNOTOriginOrDiagonal`
  (params (x :type Integer) (y :type Integer))
  (returns (NOTOriginOrDiagonal :type Boolean))
  (return (or (and (== 0 (`local.x`)) (== (`local.y`) 0)) (and (!= 0 (`local.x`)) (!= (`local.y`) 0)))))

(fn `SetGridPosition`
  (params (NewPosition :type "Vector2D Structure"))
  (set `self.GridPosition` NewPosition))

(fn `SetWorldPositionFromGridPosition`
  (locals (CurrentGridPosition :type Boolean))
  (bind (_gridposition_x _gridposition_y) (`KismetMathLibrary.BreakVector2D` (`self.GridPosition`)))
  (bind _grid (`self.Grid`))
  (bind (_returnvalue_x _returnvalue_y _returnvalue_z) (`KismetMathLibrary.BreakVector` (`Actor.K2_GetActorLocation` _grid)))
  (`/Engine/EditorBlueprintResources/StandardMacros.IsValid` _grid
    (:`Is Valid`
      (bind (_isvalid _gridlocation) (`/Game/MyContent/Blueprints_New/BP_Grid.Tile To Grid World Location` _grid (`KismetMathLibrary.FTrunc` _gridposition_x) (`KismetMathLibrary.FTrunc` _gridposition_y) true))
      (if _isvalid
        (`Actor.K2_SetActorLocation` (`self.GetOwner`) (`KismetMathLibrary.MakeVector` (`KismetMathLibrary.BreakVector2D` _gridlocation) (`.Y` (`KismetMathLibrary.BreakVector2D` _gridlocation)) _returnvalue_z) false false)))))