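; Actor component that tracks an owning actor's health and death state, broadcasting hit and death notifications.
; TakeDamage subtracts damage, calls OnHit and, at zero or below, sets IsDead and calls OnDeath.
; RepNotify handlers on CurrentHealth and IsDead repeat those notifications and the death check, with debug prints of hits.
; A separate TakenDamage event only subtracts health, leaving reactions to the RepNotify.
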(event `TakenDamage`
  (params (Damage :type Integer))
  (set `self.CurrentHealth` (- (`self.CurrentHealth`) Damage)))

(fn `OnRep_CurrentHealth`
  (bind _currenthealth (`self.CurrentHealth`))
  (`self.OnHit`)
  (`KismetSystemLibrary.PrintString` (`KismetTextLibrary.Conv_TextToString` (`|FormatText` "Hit by {name}! Remaining Health: {x}" (`KismetSystemLibrary.GetDisplayName` (`self.GetOwner`)) _currenthealth)))
  (if (<= _currenthealth 0)
    (set `self.IsDead` true)))

(fn `OnRep_IsDead`
  (if (`self.IsDead`)
    (`self.OnDeath`)))

(fn `TakeDamage`
  (params (Damage :type Integer))
  (bind _output_get (set `self.CurrentHealth` (- (`self.CurrentHealth`) (`local.Damage`))))
  (`self.OnHit`)
  (`KismetSystemLibrary.PrintString` "Been Hit")
  (if (<= _output_get 0)
    (set `self.IsDead` true)
    (`self.OnDeath`)))