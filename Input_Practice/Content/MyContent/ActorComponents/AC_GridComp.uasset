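; Actor component that places its owner on the level's BP_Grid and answers tile queries for range and attack targeting.
; On BeginPlay it finds the grid, stores the owner's tile and snaps the owner to that tile's center.
; Surrounding-tile queries gather tiles within a circular distance of an origin.
; Attack queries pick the cardinal direction nearest the mouse by dot product, then rotate an up-facing tile pattern onto the owner's tile.
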(event `self.ReceiveBeginPlay`
  (set `self.Owner` (`self.GetOwner`))
  (bind _returnvalue (`GameplayStatics.GetActorOfClass` "/Game/MyContent/Blueprints_New/BP_Grid.BP_Grid_C"))
  (set `self.Grid` _returnvalue)
  (`self.SetGridPosition` (`self.GetCurrentLocationToTile`))
  (`self.SetWorldPositionFromGridPosition`))

(fn `GetAttackableTiles`
  (params (AffectedTiles_UpDirection :type "Array of Vector2D Structure") (MousePosition :type "Vector Structure"))
  (returns (TileLocations :type "Array of Vector2D Structure"))
  (locals (IsNorth :type Boolean) (IsEast :type Boolean) (Direction :type "/Game/MyContent/Core/E_Cardinals Enum") (CardinalDirections :type "Map of Vector2D Structure to /Game/MyContent/Core/E_Cardinals Enum") (ClosestDot :type "Float (double-precision)" :default -2.0) (ClosestV2Direction :type "Vector2D Structure"))
  (bind (_value _returnvalue) (`BlueprintMapLibrary.Map_Find` (`local.CardinalDirections`) (`local.ClosestV2Direction`)))
  (bind _keys (`BlueprintMapLibrary.Map_Keys` (`local.CardinalDirections`)))
  (set `local.ClosestDot` -2.0)
  (for _array_element _keys
    (bind _returnvalue_2 (`KismetMathLibrary.DotProduct2D` (`KismetMathLibrary.Normal2D` (`KismetMathLibrary.Conv_VectorToVector2D` (- MousePosition (`Actor.K2_GetActorLocation` (`self.GetOwner`))))) _array_element))
    (if (> _returnvalue_2 (`local.ClosestDot`))
      (set `local.ClosestDot` _returnvalue_2)
      (set `local.ClosestV2Direction` _array_element)))
  (if _returnvalue
    (bind _newgridpositions (`self.RotatePositionsThenApplyOrigin` (`local.AffectedTiles_UpDirection`) (`self.GetCurrentLocationToTile`) _value))
    (return _newgridpositions)))

(fn `GetCurrentGridPosition`
  (returns (GridPosition :type "Vector2D Structure"))
  (return (`self.GridPosition`)))

(fn `GetCurrentLocationToTile`
  (returns (GridLocation :type "Vector2D Structure"))
  (bind _grid (`self.Grid`))
  (`/Engine/EditorBlueprintResources/StandardMacros.IsValid` _grid
    (:`Is Valid`
      (bind (_isvalid _row _column) (`/Game/MyContent/Blueprints_New/BP_Grid.LocationToTile` _grid (`Actor.K2_GetActorLocation` (`self.Owner`))))
      (if _isvalid
        (return (`KismetMathLibrary.MakeVector2D` (`KismetMathLibrary.Conv_IntToDouble` _row) (`KismetMathLibrary.Conv_IntToDouble` _column)))
        (else
          (`KismetSystemLibrary.PrintString` "ACTOR is not in valid location for grid ref"))))))

(fn `GetGrid`
  (returns (Grid :type "/Game/MyContent/Blueprints_New/BP_Grid Object Reference"))
  (return (`self.Grid`)))

(fn `GetSurroundingTiles`
  (params (Range :type Integer) (`IsCurrentPosOrigin?` :type Boolean))
  (returns (`Tile Locations` :type "Array of Vector2D Structure"))
  (locals (TileArray :type "Array of Vector2D Structure") (NegativeRange :type Integer) (XValue :type Integer) (YValue :type Integer) (TempGridPosition :type "Vector2D Structure") (Origin :type "Vector2D Structure"))
  (bind (_origin_x _origin_y) (`KismetMathLibrary.BreakVector2D` (`local.Origin`)))
  (if `IsCurrentPosOrigin?`
    (set `local.Origin` (`self.GetCurrentLocationToTile`))
    (else
      (set `local.Origin` (`self.GridPosition`))))
  (`KismetArrayLibrary.Array_Add` (`local.TileArray`) (`local.Origin`))
  (bind _output_get (set `local.NegativeRange` (* -1 (`local.Range`))))
  (for _index (range _output_get (+ (`local.Range`) 1))
    (set `local.XValue` _index)
    (for _index_2 (range (`local.NegativeRange`) (+ (`local.Range`) 1))
      (set `local.YValue` _index_2)
      (bind _output_get_2 (set `local.TempGridPosition` (`KismetMathLibrary.MakeVector2D` (+ _origin_x (`local.XValue`)) (+ _origin_y (`local.YValue`)))))
      (bind _returnvalue (`KismetMathLibrary.Distance2D` _output_get_2 (`local.Origin`)))
      (if (and (> _returnvalue 0.0) (<= _returnvalue (`local.Range`)))
        (if (not (`KismetArrayLibrary.Array_Contains` (`local.TileArray`) (`local.TempGridPosition`)))
          (`KismetArrayLibrary.Array_Add` (`local.TileArray`) (`local.TempGridPosition`))))))
  ;[0.05208 0.05208 0.05208 1 12] Runs when all Tiles have been checked
  (return (`local.TileArray`)))

(fn `IsNOTOriginOrDiagonal`
  (params (x :type Integer) (y :type Integer))
  (returns (NOTOriginOrDiagonal :type Boolean))
  (return (or (and (== 0 (`local.x`)) (== (`local.y`) 0)) (and (!= 0 (`local.x`)) (!= (`local.y`) 0)))))

(fn `RotatePositionsThenApplyOrigin`
  (params (GridPositions :type "Array of Vector2D Structure") (Origin :type "Vector2D Structure") (RotateDirection :type "/Game/MyContent/Core/E_Cardinals Enum" :default "NewEnumerator0"))
  (returns (NewGridPositions :type "Array of Vector2D Structure"))
  (locals (Angle :type "Float (double-precision)") (NewPositions :type "Array of Vector2D Structure") (CurrentPosition :type "Vector2D Structure"))
  (bind (_currentposition_x _currentposition_y) (`KismetMathLibrary.BreakVector2D` (`local.CurrentPosition`)))
  (bind (_currentposition_x_2 _currentposition_y_2) (`KismetMathLibrary.BreakVector2D` (`local.CurrentPosition`)))
  (bind (_currentposition_x_3 _currentposition_y_3) (`KismetMathLibrary.BreakVector2D` (`local.CurrentPosition`)))
  (for _array_element GridPositions
    (set `local.CurrentPosition` _array_element)
    (switch `/Game/MyContent/Core/E_Cardinals` RotateDirection
      (:`NewEnumerator0`
        _)
      (:`NewEnumerator1`
        ;[0.05208 0.05208 0.05208] South
        (set `local.CurrentPosition` (`KismetMathLibrary.MakeVector2D` (* _currentposition_x_2 -1.0) (* _currentposition_y_2 -1.0))))
      (:`NewEnumerator2`
        ;[0.05208 0.05208 0.05208] East
        (set `local.CurrentPosition` (`KismetMathLibrary.MakeVector2D` _currentposition_y_3 (* _currentposition_x_3 -1.0))))
      (:`NewEnumerator3`
        ;[0.05208 0.05208 0.05208] West
        (set `local.CurrentPosition` (`KismetMathLibrary.MakeVector2D` (* _currentposition_y -1.0) _currentposition_x))))
    (bind _output_get (set `local.CurrentPosition` (+ (`local.CurrentPosition`) (`local.Origin`))))
    (`KismetArrayLibrary.Array_Add` (`local.NewPositions`) _output_get))
  (return (`local.NewPositions`)))

(fn `SetGridPosition`
  (params (NewPosition :type "Vector2D Structure"))
  (set `self.GridPosition` NewPosition))

(fn `SetWorldPositionFromCurrentPosition`
  (bind (_gridlocation_x _gridlocation_y) (`KismetMathLibrary.BreakVector2D` (`self.GetCurrentLocationToTile`)))
  (bind _grid (`self.Grid`))
  (bind (_returnvalue_x _returnvalue_y _returnvalue_z) (`KismetMathLibrary.BreakVector` (`Actor.K2_GetActorLocation` _grid)))
  (`/Engine/EditorBlueprintResources/StandardMacros.IsValid` _grid
    (:`Is Valid`
      (bind (_isvalid _gridlocation) (`/Game/MyContent/Blueprints_New/BP_Grid.Tile To Grid World Location` _grid (`KismetMathLibrary.FTrunc` _gridlocation_x) (`KismetMathLibrary.FTrunc` _gridlocation_y) true))
      (if _isvalid
        (`Actor.K2_SetActorLocation` (`self.GetOwner`) (`KismetMathLibrary.MakeVector` (`KismetMathLibrary.BreakVector2D` _gridlocation) (`.Y` (`KismetMathLibrary.BreakVector2D` _gridlocation)) _returnvalue_z) false false)))))

(fn `SetWorldPositionFromGridPosition`
  (locals (CurrentGridPosition :type Boolean))
  (bind (_gridposition_x _gridposition_y) (`KismetMathLibrary.BreakVector2D` (`self.GridPosition`)))
  (bind _grid (`self.Grid`))
  (bind (_returnvalue_x _returnvalue_y _returnvalue_z) (`KismetMathLibrary.BreakVector` (`Actor.K2_GetActorLocation` _grid)))
  (`/Engine/EditorBlueprintResources/StandardMacros.IsValid` _grid
    (:`Is Valid`
      (bind (_isvalid _gridlocation) (`/Game/MyContent/Blueprints_New/BP_Grid.Tile To Grid World Location` _grid (`KismetMathLibrary.FTrunc` _gridposition_x) (`KismetMathLibrary.FTrunc` _gridposition_y) true))
      (if _isvalid
        (`Actor.K2_SetActorLocation` (`self.GetOwner`) (`KismetMathLibrary.MakeVector` (`KismetMathLibrary.BreakVector2D` _gridlocation) (`.Y` (`KismetMathLibrary.BreakVector2D` _gridlocation)) _returnvalue_z) false false)))))