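; Actor component that tracks an actor's health, damage and death.
; Health starts at the maximum on BeginPlay, and both the TakenDamage event and TakeDamage function subtract damage from it.
; RepNotify on current health fires OnHit, prints a hit message and sets IsDead at zero or below, whose own RepNotify fires OnDeath.
; Getters expose current and maximum health.
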(event `self.ReceiveBeginPlay`
  (set `self.CurrentHealth` (`self.MaxHealth`)))

(event `TakenDamage`
  (params (Damage :type Integer))
  (set `self.CurrentHealth` (- (`self.CurrentHealth`) Damage)))

(fn `GetCurrentHealth`
  (returns (CurrentHealth :type Integer))
  (return (`self.CurrentHealth`)))

(fn `GetMaxHealth`
  (returns (MaxHealth :type Integer))
  (return (`self.MaxHealth`)))

(fn `OnRep_CurrentHealth`
  (bind _currenthealth (`self.CurrentHealth`))
  (`self.OnHit`)
  (`KismetSystemLibrary.PrintString` (`KismetTextLibrary.Conv_TextToString` (`|FormatText` "Hit by {name}! Remaining Health: {x}" (`KismetSystemLibrary.GetDisplayName` (`self.GetOwner`)) _currenthealth)))
  (if (<= _currenthealth 0)
    (set `self.IsDead` true)))

(fn `OnRep_IsDead`
  (if (`self.IsDead`)
    (`self.OnDeath`)))

(fn `TakeDamage`
  (params (Damage :type Integer))
  (set `self.CurrentHealth` (- (`self.CurrentHealth`) (`local.Damage`))))