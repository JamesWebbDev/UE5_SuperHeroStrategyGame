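; Actor component that holds a unit's list of attacks and tracks the selected one for grid-based combat.
; BeginPlay checks the list against a size cap, but assigns the first entry as selected only when the list is empty.
; SetNewAttack switches selection by index and broadcasts the change.
; Getters forward the selected attack's info, damage, grid tiles or target range for AOE and single-target attacks, and animation with execute delay.
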(event `self.ReceiveBeginPlay`
  (bind _returnvalue (`KismetArrayLibrary.Array_Length` (`self.AttackList`)))
  (if (<= _returnvalue (`self.ListMax`))
    (if (== 0 _returnvalue)
      (set `self.SelectedAttack` (`|GetArrayItem` (`self.AttackList`))))
    (else
      (`KismetSystemLibrary.PrintString` "Instance of AttackList holds too many Attacks." true true (struct :`R` 1.0 :`G` 0.009102 :`B` 0.209541 :`A` 1.0) 5.0))))

(fn `GetAttackAnimation`
  (returns (Animation :type "AnimInstance Class Reference") (ExecuteDelay :type "Float (double-precision)"))
  (bind (_animation__wizard_ _executedelay) (`/Game/MyContent/Attacks/DA_Attack.GetAnimation` (`self.SelectedAttack`)))
  (return _animation__wizard_ _executedelay))

(fn `GetAttackAtIndex`
  (params (Index :type Integer))
  (returns (IsValid :type Boolean) (Attack :type "/Game/MyContent/Attacks/DA_Attack Object Reference"))
  (bind _output (`|GetArrayItem` (`self.AttackList`) Index))
  (`/Engine/EditorBlueprintResources/StandardMacros.IsValid` _output
    (:`Is Valid`
      (return true _output))
    (:`Is Not Valid`
      (return false null))))

(fn `GetAttackDamageValue`
  (returns (Damage :type Integer))
  (return (`/Game/MyContent/Attacks/DA_Attack.GetDamage` (`self.SelectedAttack`))))

(fn `GetAttackGridPositions`
  (returns (AttackableGridPosition :type "Array of Vector2D Structure"))
  (return (`/Game/MyContent/Attacks/DA_Attack.GetGridAttackTiles` (`self.SelectedAttack`))))

(fn `GetAttackInfo`
  (returns (Name :type Text) (Description :type Text))
  (bind (_name _description) (`/Game/MyContent/Attacks/DA_Attack.GetInfo` (`self.SelectedAttack`)))
  (return _name _description))

(fn `GetAttackListLength`
  (returns (ReturnValue :type Integer))
  (return (`KismetArrayLibrary.Array_Length` (`self.AttackList`))))

(fn `GetAttackValues_AOE`
  (returns (Damage :type Integer) (GridPositions :type "Array of Vector2D Structure"))
  (bind _selectedattack (`self.SelectedAttack`))
  (return (`/Game/MyContent/Attacks/DA_Attack.GetDamage` _selectedattack) (`/Game/MyContent/Attacks/DA_Attack.GetGridAttackTiles` _selectedattack)))

(fn `GetAttackValues_SingleTarget`
  (returns (Damage :type Integer) (AttackRange :type Integer))
  (bind _selectedattack (`self.SelectedAttack`))
  (return (`/Game/MyContent/Attacks/DA_Attack.GetDamage` _selectedattack) (`/Game/MyContent/Attacks/DA_Attack.GetTargetRange` _selectedattack)))

(fn `IsAttackAOE`
  (returns (IsAOE :type Boolean))
  (return (`/Game/MyContent/Attacks/DA_Attack.GetIsAOE` (`self.SelectedAttack`))))

(fn `SetNewAttack`
  (params (NewAttackIndex :type Integer))
  (if (< NewAttackIndex (`KismetArrayLibrary.Array_Length` (`self.AttackList`)))
    (bind _output_get (set `self.SelectedAttack` (`|GetArrayItem` (`self.AttackList`) (`local.NewAttackIndex`))))
    (`self.NewAttackSet` _output_get)
    (else
      (`KismetSystemLibrary.PrintString` "ERROR: New Attack Index falls out of scope of Attack List" true true (struct :`R` 1.0 :`B` 0.00687 :`A` 1.0) 10.0))))