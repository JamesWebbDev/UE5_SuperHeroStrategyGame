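; BP_AttackComponent is an actor component that holds an owner's list of attacks and tracks which one is selected.
; On BeginPlay it selects the first attack in the list, and SetNewAttack switches by index, printing an error when the index exceeds the list.
; Getters expose the list length and the selected attack's name, damage and affected grid tiles, stored as an upward-facing pattern.
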(event `self.ReceiveBeginPlay`
  (set `self.SelectedAttack` (`|GetArrayItem` (`self.AttackList`))))

(fn `GetAttackDamageValue`
  (returns (Damage :type Integer))
  (return (`.Damage_5_71CEF17D430908A5B3241D862550CC46` (break `/Game/MyContent/Blueprints_New/S_Attack` (`self.SelectedAttack`)))))

(fn `GetAttackGridPositions`
  (returns (AttackableGridPosition :type "Array of Vector2D Structure"))
  (return (`.AffectedTilesUpward_9_5E16371644BC7FBA5F51E3B21C500743` (break `/Game/MyContent/Blueprints_New/S_Attack` (`self.SelectedAttack`)))))

(fn `GetAttackListLength`
  (returns (ReturnValue :type Integer))
  (return (`KismetArrayLibrary.Array_Length` (`self.AttackList`))))

(fn `GetAttackName`
  (returns (Name :type String))
  (return (`.Name_2_E03C6C7C4412BD8B63B52B99289EC398` (break `/Game/MyContent/Blueprints_New/S_Attack` (`self.SelectedAttack`)))))

(fn `SetNewAttack`
  (params (NewAttackIndex :type Integer))
  (if (< NewAttackIndex (`KismetArrayLibrary.Array_Length` (`self.AttackList`)))
    (set `self.SelectedAttack` (`|GetArrayItem` (`self.AttackList`) (`local.NewAttackIndex`)))
    (else
      (`KismetSystemLibrary.PrintString` "ERROR: New Attack Index falls out of scope of Attack List" true true (struct :`R` 1.0 :`B` 0.00687 :`A` 1.0) 10.0))))