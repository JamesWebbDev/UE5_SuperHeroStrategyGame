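; Actor component that represents a user in a networked, turn-based grid tactics game, holding turn state, selected character and grid reference.
; Client turn events toggle tile highlights as turns and action states change.
; Server move, attack and pass events act on the GameMode's selected character, then end the user's turn.
; Attacks relay start/stop via character multicasts and resolve AOE or single-tile hits only with authority.
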(event `self.ReceiveBeginPlay`
  ;[0.04688 0.04688 0.04688 1 36] Begin Play
  (bind _returnvalue (`GameplayStatics.GetActorOfClass` "/Game/MyContent/Blueprints_New/BP_Grid.BP_Grid_C"))
  (set `self.Grid` _returnvalue))

(event `ServerAction - Move`
  (params (ActionType :type "E_PlayerActions Enum" :default "PA_Pass") (GridPosition :type "Vector2D Structure") (MoveLocation :type "Vector Structure"))
  (bind _astop_down_game_mode (cast `/Game/MyContent/Core/TopDownGameMode` (`GameplayStatics.GetGameMode`) :!pure true))
  (bind _selectedcharacter (`/Game/MyContent/Core/TopDownGameMode.GetSelectedCharacterOLD` _astop_down_game_mode))
  ;[0.04688 0.04688 0.04688 1 36] Controlling Units Logic
  ;;[0.03646 0.03646 0.03646] Add actions before the turn cycles again!  (IN C++)
  (set `self.ActionType` ActionType)
  (`AICharacter.Event_MultiRPC_SetTargetPosition` _selectedcharacter MoveLocation)
  (`AICharacter.Event_MultiRPC_ActionTaken` _selectedcharacter false)
  (`CPP_TopDownGameMode.EndUserTurn` _astop_down_game_mode (`self.ActionType`) :!label _label))

(event `StartAttackingValues SERVER`
  (params (SelectedCharacter :type "/Game/MyContent/Blueprints_New/BP_AICharacter Object Reference") (Attack :type "DA_Attack Object Reference") (CursorPos :type "Vector Structure"))
  ;[0.05208 0.05208 0.05208 1 36] Network Attack Logic
  ;;[0.05729 0.05729 0.05729] Called From Grid User
  (`/Game/MyContent/Blueprints_New/BP_AICharacter.StartAttackAndSetValues MULTI` SelectedCharacter Attack CursorPos))

(event `AttackStarting`
  ;[0.05208 0.05208 0.05208 1 36] Network Attack Logic
  ;;[0.04688 0.04688 0.04688] Called from SelectedUnit
  (`self.AttackStarting SERVER`))

(event `AttackEnding`
  (params (AttackingCharacter :type "/Game/MyContent/Blueprints_New/BP_AICharacter Object Reference"))
  ;[0.05208 0.05208 0.05208 1 36] Network Attack Logic
  ;;[0.04688 0.04688 0.04688] Called from SelectedUnit
  (`self.AttackEnding SERVER` AttackingCharacter))

(event `ServerAction - Attack`
  (params (ActionType :type "E_PlayerActions Enum" :default "PA_Pass") (AttackedPositions :type "Array of Vector2D Structure") (Damage :type Integer))
  (bind _selectedcharacter (`/Game/MyContent/Core/TopDownGameMode.GetSelectedCharacterOLD` (cast `/Game/MyContent/Core/TopDownGameMode` (`GameplayStatics.GetGameMode`) :!pure true)))
  ;[0.04688 0.04688 0.04688 1 36] Controlling Units Logic
  ;;[0.03646 0.03646 0.03646] Add actions before the turn cycles again!  (IN C++)
  (set `self.ActionType` ActionType)
  (`AICharacter.AttackPositions` _selectedcharacter AttackedPositions Damage)
  (`AICharacter.Event_MultiRPC_ActionTaken` _selectedcharacter true :!label _label_2)
  (goto _label))

(event `AttackThisFrame`
  (params (AttackingCharacter :type "/Game/MyContent/Blueprints_New/BP_AICharacter Object Reference") (Attack :type "DA_Attack Object Reference") (CursorPos :type "Vector Structure"))
  ;[0.05208 0.05208 0.05208 1 36] Network Attack Logic
  ;;[0.04688 0.04688 0.04688] Called from SelectedUnit
  (`/Engine/EditorBlueprintResources/ActorComponentMacros.Switch Has Authority`
    (:`Authority`
      (`self.ExecuteAttackOnServer` AttackingCharacter Attack CursorPos))))

(event `ServerAction - Pass`
  (params (ActionType :type "E_PlayerActions Enum" :default "PA_Pass"))
  ;[0.04688 0.04688 0.04688 1 36] Controlling Units Logic
  ;;[0.03646 0.03646 0.03646] Add actions before the turn cycles again!  (IN C++)
  (set `self.ActionType` ActionType)
  (goto _label_2))

(event `AttackStarting SERVER`
  ;[0.05208 0.05208 0.05208 1 36] Network Attack Logic
  ;;[0.05208 0.05208 0.05208] GameMode relevant Functions
  (bind _astop_down_game_mode (cast `/Game/MyContent/Core/TopDownGameMode` (`GameplayStatics.GetGameMode`)))
  (`CPP_TopDownGameMode.EndUserTurn` _astop_down_game_mode "PA_Pass"))

(event `StartTurn CLIENT`
  (params (SelectedCharacter :type "/Game/MyContent/Blueprints_New/BP_AICharacter Object Reference"))
  (bind _grid (`self.Grid`))
  ;[0.04688 0.04688 0.04688 1 36] Controlling Units Logic
  ;;[0.04167 0.04167 0.04167] Starting And Ending Turns (Client Side)  (IN C++)
  (bind _selected (`self.SetSelectedCharacter` SelectedCharacter))
  (`CPP_Grid.SetMoveableTilesState` _grid true)
  (`CPP_Grid.SetSelectedTileState` _grid true)
  (`self.SetIsMyTurn` true)
  (`AICharacter.ActivateMoveableTiles` _selected))

(event `AttackEnding SERVER`
  (params (AttackingCharacter :type "/Game/MyContent/Blueprints_New/BP_AICharacter Object Reference"))
  ;[0.05208 0.05208 0.05208 1 36] Network Attack Logic
  ;;[0.05208 0.05208 0.05208] GameMode relevant Functions
  (`/Game/MyContent/Blueprints_New/BP_AICharacter.StopAttack MULTI` AttackingCharacter)
  (bind _astop_down_game_mode (cast `/Game/MyContent/Core/TopDownGameMode` (`GameplayStatics.GetGameMode`)))
  (`CPP_TopDownGameMode.CharacterFinalActionHasConcluded` _astop_down_game_mode))

(event `EndTurn CLIENT`
  (bind _grid (`self.Grid`))
  ;[0.04688 0.04688 0.04688 1 36] Controlling Units Logic
  ;;[0.04167 0.04167 0.04167] Starting And Ending Turns (Client Side)  (IN C++)
  (`self.SetSelectedCharacter` null)
  (`CPP_Grid.SetMoveableTilesState` _grid false)
  (`CPP_Grid.SetSelectedTileState` _grid false)
  (`self.SetIsMyTurn` false))

(event `StateToggle`
  (params (NewState :type "E_PlayerActions Enum" :default "PA_Pass"))
  ;[0.04688 0.04688 0.04688 1 36] Controlling Units Logic
  ;;[0.05208 0.05208 0.05208] Changing Turn State (Client Side) (IN C++)
  (bind _output_get (set `self.CurrentState` NewState))
  (`CPP_Grid.SetHighlightedTilesState` (`self.Grid`) _output_get (`self.SelectedCharacter`)))

(fn `ExecuteAttackOnServer`
  (params (AttackingCharacter :type "/Game/MyContent/Blueprints_New/BP_AICharacter Object Reference") (Attack :type "DA_Attack Object Reference") (CursorPos :type "Vector Structure"))
  (bind _attack (`local.Attack`))
  (if (`DA_Attack.GetisAOE` Attack)
    ;[0.05208 0.05208 0.05208] AOE Attack
    (bind _outtiles (`AComp_Grid.GetAttackableTiles` (`AICharacter.GridComponent` (`local.AttackingCharacter`)) (`DA_Attack.GetAttackTiles` _attack) (`local.CursorPos`)))
    (`self.ServerAction - Attack` "PA_Attack" _outtiles (`DA_Attack.GetDamage` _attack))
    (else
      ;[0.05208 0.05208 0.05208] Single-target Attack
      (bind (_outworldposition _outgridposition) (`CPP_Grid.VectorToTile` (`self.Grid`) (`local.CursorPos`)))
      (`self.ServerAction - Attack` "PA_Attack" (`|MakeArray` _outgridposition) (`DA_Attack.GetDamage` (`local.Attack`))))))

(fn `Get Selected Character`
  (returns (SelectedCharacter :type "/Game/MyContent/Blueprints_New/BP_AICharacter Object Reference"))
  (return (`self.SelectedCharacter`)))

(fn `GetCurrentState`
  (returns (CurrentState :type "E_PlayerActions Enum"))
  (return (`self.CurrentState`)))

(fn `GetGrid`
  (returns (Grid :type "/Game/MyContent/Blueprints_New/BP_Grid Object Reference"))
  (return (`self.Grid`)))

(fn `GetHasPerformedFinalInput`
  (returns (HasPerformedFinalInput :type Boolean))
  (return (`self.HasPerformedFinalInput`)))

(fn `GetIsMyTurn`
  (returns (IsMyTurn :type Boolean))
  (return (`self.IsMyTurn`)))

(fn `GetUserIndex`
  (returns (UserIndex :type Integer))
  (return (`self.UserIndex`)))

(fn `SetHasPerformedFinalInput`
  (params (NewValue :type Boolean))
  (set `self.HasPerformedFinalInput` NewValue))

(fn `SetIsMyTurn`
  (params (NewValue :type Boolean))
  (set `self.HasPerformedFinalInput` false)
  (bind _output_get (set `self.IsMyTurn` NewValue))
  (`self.OnMyTurnChanged` _output_get))

(fn `SetSelectedCharacter`
  (params (Character :type "/Game/MyContent/Blueprints_New/BP_AICharacter Object Reference"))
  (returns (Selected :type "/Game/MyContent/Blueprints_New/BP_AICharacter Object Reference"))
  (bind _output_get (set `self.SelectedCharacter` Character))
  (return _output_get))

(fn `SetUserIndex`
  (params (NewIndex :type Integer))
  (set `self.UserIndex` NewIndex))