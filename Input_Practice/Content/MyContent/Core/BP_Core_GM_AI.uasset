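; Game mode for a turn-based grid match against AI, which spawns an AI user and starts play after a short delay.
; An event-driven loop gets the next character from the game state, signals its owning user, and advances when its action concludes or the user passes.
; Destroying a user's last character ends the match and notifies players.
; Player starts are mapped by player index and chosen by player count.
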(event `self.ReceiveBeginPlay`
  ;[0.05208 0.05208 0.05208 1 28] Begin/PostLogin
  (`|ExecutionSequence`
    (:`then_0`
      (bind _returnvalue (`GameplayStatics.GetActorOfClass` "/Game/MyContent/Blueprints/BP_Grid.BP_Grid_C"))
      (set `self.Grid` _returnvalue))
    (:`then_1`
      (bind _asbp_core_gs (cast `/Game/MyContent/Core/BP_Core_GS` (`GameplayStatics.GetGameState`)))
      (bind _output_get (set `self.TopDownGameState` _asbp_core_gs))
      (`CPP_TopDownGameState.InitialiseCharacters` _output_get))))

(event `self.StartGameWithAI`
  ;[0.05208 0.05208 0.05208 1 28] Begin/PostLogin
  (bind _out_ai (`self.Spawn AI Grid User`))
  (bind _asgrid_user (cast `GridUser` _out_ai))
  (`AComp_GridUser.SetUserIndex` (`GridUser.GetGridUser` _asgrid_user) 1)
  (`/Game/MyContent/Core/BP_Core_GS.InitialiseOwnersOnAllCharacters` (`self.TopDownGameState`))
  (`KismetSystemLibrary.PrintText` (`|FormatText` "Starting Game in {x} seconds!" 3.0) true true (struct :`G` 0.66 :`B` 1.0 :`A` 1.0) 5.0)
  ;;[0.05729 0.05729 0.05729 1 14] Allow Player to fully construct before proceeding
  (`KismetSystemLibrary.Delay` 3.0)
  (`self.StartGame`))

(event `self.StartGame`
  (bind _griduser (`self.GetUserInTurn`))
  ;[0.05729 0.05729 0.05729 1 28] Game Flow
  (set `self.HasGameStarted` true)
  (set `self.IsGameOver` false)
  (`/Game/MyContent/Core/BP_Core_GS.EnablePlayerGameplayUI` (`self.TopDownGameState`))
  (if (not (`self.IsGameOver`)) :!label _label
    (`self.SetNextActiveCharacterAndPlayer`)
    (add `/Game/MyContent/Blueprints/BP_AICharacter.OnActionConcluded` (`self.SelectedCharacter`) (delegate `self.CharacterFinalActionHasConcluded`))
    (`/Engine/EditorBlueprintResources/StandardMacros.IsValid` _griduser
      (:`Is Valid`
        (`AComp_GridUser.Event_ClientRPC_StartTurn` _griduser (`self.SelectedCharacter`)))
      (:`Is Not Valid`
        (`KismetSystemLibrary.PrintString` "Nope")))))

(event `self.CharacterFinalActionHasConcluded`
  ;[0.05729 0.05729 0.05729 1 28] Game Flow
  (remove `/Game/MyContent/Blueprints/BP_AICharacter.OnActionConcluded` (`self.SelectedCharacter`) (delegate `self.CharacterFinalActionHasConcluded`))
  (goto _label))

(event `self.EndGame`
  (params (WinningPlayerIndex :type Integer))
  ;[0.05729 0.05729 0.05729 1 28] Game Flow
  (for (_array_element _array_index) (`CPP_TopDownGameState.GridUserList` (`self.TopDownGameState`))
    (bind _asbp_user_player (cast `/Game/MyContent/Blueprints/BP_User_Player` _array_element))
    (`/Game/MyContent/Blueprints/BP_User_Player.GameOver` _asbp_user_player (== _array_index WinningPlayerIndex))))

(event `self.EndUserTurn`
  (params (EndingUserState :type "E_PlayerActions Enum" :default "PA_Pass"))
  ;[0.04688 0.04688 0.04688 1 28] Player Turn Flow
  (`AComp_GridUser.Event_ClientRPC_EndTurn` (`self.GetUserInTurn`))
  (if (`|EnumEquality` EndingUserState "PA_Pass")
    (`KismetSystemLibrary.Delay` 1.0)
    (`self.CharacterFinalActionHasConcluded`)))

(event `self.DestroyCharacter`
  (params (InCharacter :type "AICharacter Object Reference") (OwningPlayerIndex :type Integer))
  (bind _topdowngamestate (`self.TopDownGameState`))
  ;[0.04688 0.04688 0.04688 1 28] Player Turn Flow
  (`CPP_TopDownGameState.RemoveCharacterFromList` _topdowngamestate InCharacter)
  (`self.K2_DestroyActor` InCharacter)
  (bind _returnvalue (`CPP_TopDownGameState.GetCharactersOwnedByPlayers` _topdowngamestate OwningPlayerIndex))
  (if (== (`KismetArrayLibrary.Array_Length` _returnvalue) 0)
    (set `self.IsGameOver` true)
    (`self.EndGame` (`AICharacter.GetPlayerIndex` (`|GetArrayItem` (`CPP_TopDownGameState.CharacterList` _topdowngamestate))))))

(fn `ChoosePlayerStart`
  (params (Player :type "Controller Object Reference"))
  (returns (ReturnValue :type "Actor Object Reference"))
  (`self.InitialiseSpawnPoints (If Needed)`)
  (bind _returnvalue (`self.GetNumPlayers`))
  (bind (_value _returnvalue_2) (`BlueprintMapLibrary.Map_Find` (`self.SpawnPoints`) _returnvalue))
  (if _returnvalue_2
    (return _value)))

(fn `GetUserInTurn`
  (returns (GridUser :type "AComp_GridUser Object Reference"))
  (bind _returnvalue (`CPP_TopDownGameState.GetUserByIndex` (`self.TopDownGameState`) (`self.CurrentPlayersTurn`)))
  (`/Engine/EditorBlueprintResources/StandardMacros.IsValid` _returnvalue
    (:`Is Valid`
      (bind _asgrid_user (cast `GridUser` _returnvalue)
        (:`then`
          (return (`GridUser.GetGridUser` _asgrid_user)))
        (:`CastFailed`
          (`KismetSystemLibrary.PrintString` "Cast Failed"))))
    (:`Is Not Valid`
      (`KismetSystemLibrary.PrintString` "User By Index Invalid"))))

(fn `InitialiseSpawnPoints (If Needed)`
  (if (== (`BlueprintMapLibrary.Map_Length` (`self.SpawnPoints`)) 0)
    (bind _outactors (`GameplayStatics.GetAllActorsOfClass` "/Game/MyContent/Core/BP_Core_PStart.BP_Core_PStart_C"))
    (for _array_element _outactors
      (`BlueprintMapLibrary.Map_Add` (`self.SpawnPoints`) (`/Game/MyContent/Core/BP_Core_PStart.GetPlayerIndex` _array_element) _array_element))))

(fn `SetNextActiveCharacterAndPlayer`
  (bind _returnvalue (`CPP_TopDownGameState.GetNextActiveCharacter` (`self.TopDownGameState`)))
  (bind _output_get (set `self.SelectedAICharacter` _returnvalue))
  (bind _asbp_aicharacter (cast `/Game/MyContent/Blueprints/BP_AICharacter` _output_get))
  (bind _output_get_2 (set `self.SelectedCharacter` _asbp_aicharacter))
  (set `self.CurrentPlayersTurn` (`AICharacter.GetPlayerIndex` _output_get_2)))

(fn `Spawn AI Grid User`
  (returns (`Out AI` :type "/Game/MyContent/Blueprints/BP_User_AI Object Reference"))
  (bind _returnvalue (`|SpawnActorFromClass` "/Game/MyContent/Blueprints/BP_User_AI.BP_User_AI_C" (`KismetMathLibrary.MakeTransform` (0.0 0.0 0.0)) "Undefined" "OverrideRootScale" null null))
  (return _returnvalue))

(fn `UserConstructionScript`)