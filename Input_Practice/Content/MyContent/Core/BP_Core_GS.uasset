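; Core game state Blueprint, judging by its GS suffix, that links player pawns and characters to their users.
; It gathers player pawns as BP_User_Player and calls StartGameplay on each to enable gameplay UI.
; Owner initialisation refreshes the grid user list, then assigns each listed character the valid user at its PlayerIndex through SetOwningUser.
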(fn `EnablePlayerGameplayUI`
  (for _array_element (`self.GetBP_Players`)
    (`/Game/MyContent/Blueprints/BP_User_Player.StartGameplay` _array_element)))

(fn `GetBP_Players`
  (returns (BP_Players :type "Array of /Game/MyContent/Blueprints/BP_User_Player Object Reference"))
  (locals (BPs :type "Array of /Game/MyContent/Blueprints/BP_User_Player Object Reference"))
  (for _array_element (`self.GetPlayerPawns`)
    (bind _asbp_user_player (cast `/Game/MyContent/Blueprints/BP_User_Player` _array_element))
    (`KismetArrayLibrary.Array_Add` (`local.BPs`) _asbp_user_player))
  (return (`local.BPs`)))

(fn `InitialiseOwnersOnAllCharacters`
  (`self.SetGridUsersList`)
  (for _array_element (`self.CharacterList`)
    (bind _output (`|GetArrayItem` (`self.GridUserList`) (`AICharacter.PlayerIndex` _array_element)))
    (`/Engine/EditorBlueprintResources/StandardMacros.IsValid` _output
      (:`Is Valid`
        (`AICharacter.SetOwningUser` _array_element _output)))))

(fn `UserConstructionScript`)